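; Laser splitter reaction that turns one beam hitting its receiver into two outgoing beams.
; Setup stores the receiver and two split components, spawning a Beam at each split along its forward vector.
; A receiver hit records the incoming beam and calls UpdateSplits, which activates both outputs in fixed red, ignoring the input color.
; Hit end only clears the stored beam, without calling UpdateSplits to deactivate the outputs.
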(event `self.ReceiveTick`
  (params (DeltaSeconds :type "Float (single-precision)")))

(event `self.ReceiveBeginPlay`)

(event `self.OnLazorHitBegin`
  (params (_hitPos :type "Vector Structure (by ref)") (_hitDir :type "Vector Structure (by ref)") (_hitComponent :type "PrimitiveComponent Object Reference") (_beam :type "Beam Object Reference"))
  (if (== _hitComponent (`self.Receiver`))
    (set `self.InBeam` _beam)
    (`self.UpdateSplits`)))

(event `self.OnLazorHitEnd`
  (params (_hitComponent :type "PrimitiveComponent Object Reference") (_beam :type "Beam Object Reference"))
  (if (== _hitComponent (`self.Receiver`))
    (if (== _beam (`self.InBeam`))
      (set `self.InBeam` (`self.NullBeam`)))))

(fn `Setup`
  (params (Split1 :type "SceneComponent Object Reference") (Split2 :type "SceneComponent Object Reference") (Receiver :type "StaticMeshComponent Object Reference"))
  (bind _split2 (`self.Split2`))
  (set `self.Receiver` Receiver)
  (set `self.Split1` Split1)
  (set `self.Split2` Split2)
  (bind _returnvalue (`|SpawnActorFromClass` "/Script/Puzzors.Beam" (`SceneComponent.K2_GetComponentToWorld` (`self.Split1`))))
  (`Beam.SetDirection` _returnvalue (`SceneComponent.GetForwardVector` (`self.Split1`)))
  (set `self.OutBeam1` _returnvalue)
  (bind _returnvalue_2 (`|SpawnActorFromClass` "/Script/Puzzors.Beam" (`SceneComponent.K2_GetComponentToWorld` _split2)))
  (`Beam.SetDirection` _returnvalue_2 (`SceneComponent.GetForwardVector` _split2))
  (set `self.OutBeam2` _returnvalue_2))