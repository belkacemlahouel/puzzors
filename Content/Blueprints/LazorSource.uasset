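; LazorSource is an actor that emits a colored laser beam from its position along its forward vector.
; On BeginPlay it spawns a Beam actor at its own transform, sets the direction and color, stores the reference and activates it.
; The Movable OnMove event re-aims the beam along the current forward vector, without updating its position or relying on Tick.
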(event `self.ReceiveBeginPlay`
  (bind _returnvalue (`|SpawnActorFromClass` "/Script/Puzzors.Beam" (`self.GetTransform`) true))
  (`Beam.SetDirection` _returnvalue (`KismetMathLibrary.GetForwardVector` (`self.K2_GetActorRotation`)))
  (`Beam.SetColor` _returnvalue (`self.Color_0`))
  (bind _output_get (set `self.Beam` _returnvalue))
  (`Beam.Activate` _output_get))

(event `self.ReceiveActorBeginOverlap`
  (params (OtherActor :type "Actor Object Reference")))

(event `self.ReceiveTick`
  (params (DeltaSeconds :type "Float (single-precision)")))

(event `self.Movable.OnMove`
  (`Beam.SetDirection` (`self.Beam`) (`KismetMathLibrary.GetForwardVector` (`self.K2_GetActorRotation`))))

(fn `UserConstructionScript`)