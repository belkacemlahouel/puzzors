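; BeamSource spawns and steers a Beam, acting as the emitter for it.
; LaunchBeam spawns the Beam at the Source transform, aims it along that transform's forward vector, applies BeamColor, stores the reference and activates it.
; UpdateBeamDirection and UpdateBeamLocation then redirect or move the stored Beam without sweeping.
; The event graph does nothing, so launching and updates rely on calls to these functions.
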(event `self.ReceiveTick`
  (params (DeltaSeconds :type "Float (single-precision)")))

(event `self.ReceiveBeginPlay`)

(fn `LaunchBeam`
  (bind _returnvalue (`|SpawnActorFromClass` "/Script/Puzzors.Beam" (`self.Source`) true))
  (`Beam.SetDirection` _returnvalue (`KismetMathLibrary.GetForwardVector` (.rotation (`self.Source`))))
  (`Beam.SetColor` _returnvalue (`self.BeamColor`))
  (bind _output_get (set `self.Beam` _returnvalue))
  (`Beam.Activate` _output_get))

(fn `UpdateBeamDirection`
  (params (Direction :type "Vector Structure"))
  (`Beam.SetDirection` (`self.Beam`) Direction))

(fn `UpdateBeamLocation`
  (params (Location :type "Vector Structure"))
  (`Actor.K2_SetActorLocation` (`self.Beam`) Location false))