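; Laser concentrator logic that merges beams hitting two concentrator meshes into one output beam with their combined color.
; Setup stores both concentrators and the output, then spawns an inactive beam along the output's forward vector.
; Hit events track each concentrator's current beam, stashing displaced ones and restoring the first stashed when the current leaves.
; The output fires only while both inputs are lit, with color changes broadcast for concentrators and output.
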(event `self.ReceiveTick`
  (params (DeltaSeconds :type "Float (single-precision)")))

(event `self.ReceiveBeginPlay`)

(event `self.OnLazorHitBegin`
  (params (_hitPos :type "Vector Structure (by ref)") (_hitDir :type "Vector Structure (by ref)") (_hitComponent :type "PrimitiveComponent Object Reference") (_beam :type "Beam Object Reference"))
  (`self.IsReady`
    (:`True`
      (bind _asstatic_mesh_component (cast `StaticMeshComponent` _hitComponent))
      (`self.LazorHitBegin` _beam _asstatic_mesh_component
        (:`Out`
          (`self.UpdateBeamColor`)
          (`self.ShouldFireBeam`
            (:`True`
              (`Beam.Activate` (`self.OutBeam`)))))))))

(event `self.OnLazorHitEnd`
  (params (_hitComponent :type "PrimitiveComponent Object Reference") (_beam :type "Beam Object Reference"))
  (`self.IsReady`
    (:`True`
      (bind _asstatic_mesh_component (cast `StaticMeshComponent` _hitComponent))
      (`self.LazorHitEnd` _asstatic_mesh_component _beam
        (:`Out`
          (`self.ShouldFireBeam`
            (:`False`
              (`Beam.Deactivate` (`self.OutBeam`))
              (`self.OutColorChanged` "BC_NONE"))))))))

(fn `Setup`
  (params (Concentrator1 :type "StaticMeshComponent Object Reference") (Concentrator2 :type "StaticMeshComponent Object Reference") (Output :type "SceneComponent Object Reference"))
  (bind _output_get (set `self.Concentrator1` Concentrator1))
  (bind _output_get_2 (set `self.Concentrator2` Concentrator2))
  (bind _output_get_3 (set `self.Output` Output))
  (set `self.Ready` (and (`KismetSystemLibrary.IsValid` _output_get_3) (`KismetSystemLibrary.IsValid` _output_get_2) (`KismetSystemLibrary.IsValid` _output_get)))
  (`self.IsReady`
    (:`True`
      (if (== (`self.OutBeam`) (`self.NullBeam`))
        (bind _returnvalue (`|SpawnActorFromClass` "/Script/Puzzors.Beam" (`SceneComponent.K2_GetComponentToWorld` (`self.Output`))))
        (bind _output_get_4 (set `self.OutBeam` _returnvalue))
        (`Beam.SetDirection` _output_get_4 (`SceneComponent.GetForwardVector` (`self.Output`)))
        (`Beam.Deactivate` _output_get_4)))))

(fn `UpdateBeamColor`
  (`self.ShouldFireBeam`
    (:`True`
      _)
    (:`AlreadyFired`
      _))
  (bind _returnvalue (`Beam.Color` (`self.Beam1`)))
  (bind _returnvalue_2 (`Beam.Color` (`self.Beam2`)))
  (bind _returnvalue_3 (`Beam.AddColor` _returnvalue_2 _returnvalue))
  (`self.OutColorChanged` _returnvalue_3)
  (`Beam.SetColor` (`self.OutBeam`) _returnvalue_3))