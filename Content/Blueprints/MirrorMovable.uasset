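; MirrorMovable is a Blueprint that, judging by its name, provides a movable mirror, rotated through a single Rotate event.
; When both targets are valid, Rotate applies the delta's yaw to YawTarget and the summed pitch and roll to PitchRollTarget as relative rotations.
; The AddPitch flag selects whether that sum turns PitchRollTarget on its pitch or roll axis.
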(event `self.ReceiveTick`
  (params (DeltaSeconds :type "Float (single-precision)")))

(event `self.ReceiveBeginPlay`)

(event `self.Rotate`
  (params (_Deltas :type "Rotator Structure (by ref)"))
  (bind _returnvalue (+ (.pitch _Deltas) (.roll _Deltas)))
  (if (and (`KismetSystemLibrary.IsValid` (`self.YawTarget`)) (`KismetSystemLibrary.IsValid` (`self.PitchRollTarget`)))
    (`SceneComponent.K2_AddRelativeRotation` (`self.YawTarget`) (`KismetMathLibrary.MakeRotator` 0.0 (.yaw _Deltas)) false)
    (if (`self.AddPitch`)
      (`SceneComponent.K2_AddRelativeRotation` (`self.PitchRollTarget`) (`KismetMathLibrary.MakeRotator` _returnvalue) false)
      (else
        (`SceneComponent.K2_AddRelativeRotation` (`self.PitchRollTarget`) (`KismetMathLibrary.MakeRotator` 0.0 0.0 _returnvalue) false)))))