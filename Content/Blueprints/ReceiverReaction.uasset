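; ReceiverReaction reacts to laser beams hitting a designated Receiver component.
; When a hit begins or ends on that component, it compares the beam's color to Color0.
; A matching hit sets Active and calls OnActivate, and the end of that hit clears Active and calls OnDeactivate.
; Only the hit-begin path checks that Receiver is valid.
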(event `self.ReceiveTick`
  (params (DeltaSeconds :type "Float (single-precision)")))

(event `self.ReceiveBeginPlay`)

(event `self.OnLazorHitBegin`
  (params (_hitPos :type "Vector Structure (by ref)") (_hitDir :type "Vector Structure (by ref)") (_hitComponent :type "PrimitiveComponent Object Reference") (_beam :type "Beam Object Reference"))
  (bind _receiver (`self.Receiver`))
  (`/Engine/EditorBlueprintResources/StandardMacros.IsValid` _receiver
    (:`Is Valid`
      (if (== _hitComponent _receiver)
        (bind _returnvalue (`Beam.Color` _beam))
        (if (`|EnumEquality` _returnvalue (`self.Color_0`))
          (set `self.Active` true)
          (`self.OnActivate`))))))

(event `self.OnLazorHitEnd`
  (params (_hitComponent :type "PrimitiveComponent Object Reference") (_beam :type "Beam Object Reference"))
  (if (== _hitComponent (`self.Receiver`))
    (bind _returnvalue (`Beam.Color` _beam))
    (if (`|EnumEquality` _returnvalue (`self.Color_0`))
      (set `self.Active` false)
      (`self.OnDeactivate`))))